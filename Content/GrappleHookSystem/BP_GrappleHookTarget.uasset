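; Grapple hook target actor that marks a grapple point of one of four types: Zip to Point, Launch, Launch Up or Swing.
; The construction script sets the hook mesh, scale and offset from GrappleType, and BeginPlay creates the matching indicator widget for its Widget component.
; SetActive toggles that widget's visibility, and GetCharacterTargetLocation returns CharacterOffset transformed into world space by the actor's transform.
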(event EventBeginPlay
  (switch Utilities|FlowControl|Switch|SwitchonE_GrappleTypes (Variables|Default|GetGrappleType)
    (:NewEnumerator0
      (bind _returnvalue (UserInterface|CreateWidget "/Game/GrappleHookSystem/TargetWidgets/ZipToPoint_Widget.ZipToPoint_Widget_C"))
      (UserInterface|SetWidget (Variables|Default|GetWidget) _returnvalue))
    (:NewEnumerator1
      (bind _returnvalue_2 (UserInterface|CreateWidget "/Game/GrappleHookSystem/TargetWidgets/Launch_Widget.Launch_Widget_C"))
      (UserInterface|SetWidget (Variables|Default|GetWidget) _returnvalue_2))
    (:NewEnumerator2
      (bind _returnvalue_3 (UserInterface|CreateWidget "/Game/GrappleHookSystem/TargetWidgets/LaunchUp_Widget.LaunchUp_Widget_C"))
      (UserInterface|SetWidget (Variables|Default|GetWidget) _returnvalue_3))
    (:NewEnumerator3
      (bind _returnvalue_4 (UserInterface|CreateWidget "/Game/GrappleHookSystem/TargetWidgets/Swing_Widget.Swing_Widget_C"))
      (UserInterface|SetWidget (Variables|Default|GetWidget) _returnvalue_4))))

(fn ConstructionScript
  (bind _sm_hook (Variables|Default|GetSM_Hook))
  (bind _sm_hook_2 (Variables|Default|GetSM_Hook))
  (bind _sm_hook_3 (Variables|Default|GetSM_Hook))
  (bind _sm_hook_4 (Variables|Default|GetSM_Hook))
  (switch Utilities|FlowControl|Switch|SwitchonE_GrappleTypes (Variables|Default|GetGrappleType)
    (:NewEnumerator0
      (Components|StaticMesh|SetStaticMesh _sm_hook_2 "/Game/GrappleHookSystem/SM_ZipToPointHook.SM_ZipToPointHook")
      (Transformation|SetWorldScale3D _sm_hook_2 "1.500000,1.500000,1.500000")
      (Transformation|SetRelativeLocation _sm_hook_2 "0.000000,0.000000,-50.000000" false false))
    (:NewEnumerator1
      (Components|StaticMesh|SetStaticMesh _sm_hook_3 "/Game/GrappleHookSystem/SM_LaunchHook.SM_LaunchHook")
      (Transformation|SetWorldScale3D _sm_hook_3 "2.000000,2.000000,2.000000")
      (Transformation|SetRelativeLocation _sm_hook_3 "0.000000,0.000000,-50.000000" false false))
    (:NewEnumerator2
      (Components|StaticMesh|SetStaticMesh _sm_hook_4 "/Game/GrappleHookSystem/SM_LaunchUpHook.SM_LaunchUpHook")
      (Transformation|SetWorldScale3D _sm_hook_4 "2.000000,2.000000,2.000000")
      (Transformation|SetRelativeLocation _sm_hook_4 "0.000000,0.000000,-50.000000" false false))
    (:NewEnumerator3
      (Components|StaticMesh|SetStaticMesh _sm_hook "/Game/GrappleHookSystem/SM_SwingHook.SM_SwingHook")
      (Transformation|SetWorldScale3D _sm_hook "5.000000,5.000000,5.000000")
      (Transformation|SetRelativeLocation _sm_hook "0.000000,0.000000,-50.000000" false false))))

(fn SetActive
  (params (Active :type Boolean))
  (Rendering|SetVisibility (Variables|Default|GetWidget) Active false))

(fn GetCharacterTargetLocation
  (return (Math|Transform|TransformLocation (Transformation|GetActorTransform) (Variables|Default|GetCharacterOffset))))